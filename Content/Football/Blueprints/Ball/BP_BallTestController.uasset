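; Test controller for kicking the football, mapping gamepad face and shoulder buttons to ground, lofted and through passes, shots and curled finesse shots.
; Holding a button charges power on Tick and drives the WBP_PowerMeter widget created at BeginPlay.
; Release calls ApplyKick on the first BP_Football found, with fixed direction, lift and spin per kick type and charge-interpolated power.
; R resets the ball to the Ball_Spawn-tagged actor.
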(event EventBeginPlay
  (bind _outactors (Actor|GetAllActorsOfClass "/Game/Football/Blueprints/Ball/BP_Football.BP_Football_C"))
  (Variables|Default|SetBallRef (Utilities|Array|Get(acopy) _outactors))
  (bind _returnvalue (Class|WidgetBlueprintLibrary|Create "/Game/Football/Blueprints/UI/WBP_PowerMeter.WBP_PowerMeter_C"))
  (bind _aswbp_power_meter (Utilities|Casting|CastToWBP_PowerMeter _returnvalue))
  (Variables|Default|SetPowerMeterRef _aswbp_power_meter)
  (UserInterface|Viewport|AddtoViewport _aswbp_power_meter 0)
  (Default|HideMeter _aswbp_power_meter))

(event EventTick
  (params (DeltaSeconds :type Float%20%28single-precision%29))
  (if (Variables|Default|GetbCharging)
    (Variables|Default|SetCharge (Math|Float|Clamp(Float) (+ (Variables|Default|GetCharge) (* DeltaSeconds 0.8))))
    (Default|UpdatePower (Variables|Default|GetPowerMeterRef) (Math|Float|Clamp(Float) (+ (Variables|Default|GetCharge) (* DeltaSeconds 0.8))))))

(event Input|GamepadEvents|GamepadFaceButtonRight
  (params (Key :type Key%20Structure :default "None"))
  (:Pressed
    (Variables|Default|SetbCharging true)
    (Variables|Default|SetCharge 0.0)
    (Default|ShowMeter (Variables|Default|GetPowerMeterRef) "SHOT"))
  (:Released
    (Variables|Default|SetbCharging false)
    (Default|ApplyKick (Variables|Default|GetBallRef) "1.000000,0.030000,0.000000" (Math|Float|Lerp 2.6e+03 4.4e+03 (Variables|Default|GetCharge)) 0.22 1.2e+02 0 2e+01)
    (Default|HideMeter (Variables|Default|GetPowerMeterRef))))

(event Input|GamepadEvents|GamepadRightShoulder
  (params (Key :type Key%20Structure :default "None"))
  (:Pressed
    (Variables|Default|SetbCharging true)
    (Variables|Default|SetCharge 0.0)
    (Default|ShowMeter (Variables|Default|GetPowerMeterRef) "FINESSE R"))
  (:Released
    (Variables|Default|SetbCharging false)
    (Default|ApplyKick (Variables|Default|GetBallRef) "0.950000,0.140000,0.000000" (Math|Float|Lerp 2.2e+03 3.8e+03 (Variables|Default|GetCharge)) 0.22 1.5e+03 0 4e+01)
    (Default|HideMeter (Variables|Default|GetPowerMeterRef))))

(event Input|GamepadEvents|GamepadLeftShoulder
  (params (Key :type Key%20Structure :default "None"))
  (:Pressed
    (Variables|Default|SetbCharging true)
    (Variables|Default|SetCharge 0.0)
    (Default|ShowMeter (Variables|Default|GetPowerMeterRef) "FINESSE L"))
  (:Released
    (Variables|Default|SetbCharging false)
    (Default|ApplyKick (Variables|Default|GetBallRef) "0.950000,-0.140000,0.000000" (Math|Float|Lerp 2.2e+03 3.8e+03 (Variables|Default|GetCharge)) 0.22 -1.5e+03 0 4e+01)
    (Default|HideMeter (Variables|Default|GetPowerMeterRef))))

(event Input|KeyboardEvents|R
  (params (Key :type Key%20Structure :default "None"))
  (:Pressed
    (bind _outactors (Actor|GetAllActorswithTag "Ball_Spawn"))
    (Default|ResetBall (Variables|Default|GetBallRef) (Transformation|GetActorTransform (Utilities|Array|Get(acopy) _outactors)) false)))

(event Input|GamepadEvents|GamepadFaceButtonBottom
  (params (Key :type Key%20Structure :default "None"))
  (:Pressed
    (Variables|Default|SetbCharging true)
    (Variables|Default|SetCharge 0.0)
    (Default|ShowMeter (Variables|Default|GetPowerMeterRef) "GROUND PASS"))
  (:Released
    (Variables|Default|SetbCharging false)
    (Default|ApplyKick (Variables|Default|GetBallRef) "1.000000,0.000000,0.000000" (Math|Float|Lerp 7e+02 1.8e+03 (Variables|Default|GetCharge)) 0.02 0.0 0 (* (Math|Float|Lerp 7e+02 1.8e+03 (Variables|Default|GetCharge)) -0.52))
    (Default|HideMeter (Variables|Default|GetPowerMeterRef))))

(event Input|GamepadEvents|GamepadFaceButtonLeft
  (params (Key :type Key%20Structure :default "None"))
  (:Pressed
    (Variables|Default|SetbCharging true)
    (Variables|Default|SetCharge 0.0)
    (Default|ShowMeter (Variables|Default|GetPowerMeterRef) "LOFTED PASS"))
  (:Released
    (Variables|Default|SetbCharging false)
    (Default|ApplyKick (Variables|Default|GetBallRef) "1.000000,0.000000,0.000000" (Math|Float|Lerp 1.4e+03 2.8e+03 (Variables|Default|GetCharge)) 0.45 6e+01 0 0.0)
    (Default|HideMeter (Variables|Default|GetPowerMeterRef))))

(event Input|GamepadEvents|GamepadFaceButtonTop
  (params (Key :type Key%20Structure :default "None"))
  (:Pressed
    (Variables|Default|SetbCharging true)
    (Variables|Default|SetCharge 0.0)
    (Default|ShowMeter (Variables|Default|GetPowerMeterRef) "THROUGH BALL"))
  (:Released
    (Variables|Default|SetbCharging false)
    (Default|ApplyKick (Variables|Default|GetBallRef) "1.000000,0.030000,0.000000" (Math|Float|Lerp 1.3e+03 2.8e+03 (Variables|Default|GetCharge)) 0.12 5e+01 0 0.0)
    (Default|HideMeter (Variables|Default|GetPowerMeterRef))))

(fn ConstructionScript)