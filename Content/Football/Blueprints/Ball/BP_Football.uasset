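; Physics football actor that can be kicked with power, lift, side spin and top spin, and reset to a spawn transform.
; Tick adds a Magnus force from spin crossed with velocity while spinning and moving vertically, plus optional quadratic air drag.
; Hits on upward-facing surfaces blend horizontal spin toward a velocity-based value.
; Kicks record the last kicker and fire a kicked event, while slowing below a threshold fires a stopped event.
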(event OnComponentHit(BallSphere)
  (params (HitComponent :type Primitive%20Component%20Object%20Reference) (OtherActor :type Actor%20Object%20Reference) (OtherComp :type Primitive%20Component%20Object%20Reference) (NormalImpulse :type Vector :default "0, 0, 0") (Hit :type Hit%20Result%20Structure%20%28by%20ref%29))
  (bind _ballsphere (Variables|Default|GetBallSphere))
  (bind _addedgroundspinfriction (Variables|Default|GetAddedGroundSpinFriction))
  (bind _returnvalue (Physics|GetPhysicsAngularVelocityinDegrees _ballsphere "None"))
  (bind (_x _y _z) (Math|Vector|BreakVector _returnvalue))
  (if (> (.Z (Math|Vector|BreakVector (.ImpactNormal (Collision|BreakHitResult Hit)))) 0.7)
    (bind _returnvalue_2 (Physics|GetPhysicsLinearVelocity (Variables|Default|GetBallSphere) "None"))
    (Class|PrimitiveComponent|SetPhysicsAngularVelocityinDegrees (Variables|Default|GetBallSphere) (Math|Vector|MakeVector (+ _x (* (- (* (.X (Math|Vector|BreakVector _returnvalue_2)) 5.2e+02) _x) _addedgroundspinfriction)) (+ _y (* _addedgroundspinfriction (- (* (.Y (Math|Vector|BreakVector _returnvalue_2)) 5.2e+02) _y))) _z) false "None")))

(event EventTick
  (params (DeltaSeconds :type Float%20%28single-precision%29))
  (bind _ballsphere (Variables|Default|GetBallSphere))
  (bind _returnvalue (Physics|GetPhysicsAngularVelocityinDegrees _ballsphere "None"))
  (if (< (Math|Vector|VectorLength _returnvalue) 3e+01)
    _
    (else
      (bind _returnvalue_2 (Physics|GetPhysicsLinearVelocity (Variables|Default|GetBallSphere) "None"))
      (if (< (Math|Float|Absolute(Float) (.z _returnvalue_2)) 15.0)
        _
        (else
          (Physics|AddForce (Variables|Default|GetBallSphere) (* (Math|Vector|CrossProduct (* _returnvalue 0.01745) (Math|Vector|MakeVector (.x _returnvalue_2) (.y _returnvalue_2) (.z _returnvalue_2))) (Variables|Default|GetAddedMagnusCoef)) "None" false)))))
  (if (Variables|Default|GetAddedbAirdragEnabled)
    (bind _returnvalue_3 (Physics|GetPhysicsLinearVelocity (Variables|Default|GetBallSphere) "None"))
    (if (< (Math|Vector|VectorLength _returnvalue_3) 4e+01)
      (bind _returnvalue_4 (Physics|GetPhysicsLinearVelocity (Variables|Default|GetBallSphere) "None" :!label _label))
      (if (and (Variables|Default|GetbIsMoving) (< (Math|Vector|VectorLength _returnvalue_4) (Variables|Default|GetMinStopSpeed)))
        (Variables|Default|SetbIsMoving false)
        (Default|CallOnBallStopped)
        (elif (not (< (Math|Vector|VectorLength _returnvalue_4) (Variables|Default|GetMinStopSpeed)))
          (Variables|Default|SetbIsMoving true)))
      (else
        (Physics|AddForce (Variables|Default|GetBallSphere) (* (* (Math|Vector|Normalize _returnvalue_3) -1.0) (* (* (Math|Vector|VectorLength _returnvalue_3) (Math|Vector|VectorLength _returnvalue_3)) (Variables|Default|GetAddedAirDragCoeff))) "None" false)))
    (else
      (goto _label))))

(fn ConstructionScript)

(fn ApplyKick
  (params (KickDirection :type Vector) (Power :type Float%20%28double-precision%29) (Lift :type Float%20%28double-precision%29) (SpinRight :type Float%20%28double-precision%29) (Kicker :type Actor%20Object%20Reference) (SpinTop :type Float%20%28double-precision%29))
  (bind _returnvalue (Math|Vector|MakeVector 0.0 0.0 1.0))
  (Variables|Default|SetLastKicker Kicker)
  (Physics|SetSimulatePhysics (Variables|Default|GetBallSphere) true)
  (Physics|AddImpulse (Variables|Default|GetBallSphere) (* Power (Math|Vector|Normalize (+ (Math|Vector|Normalize KickDirection) (* Lift (Math|Vector|MakeVector 0.0 0.0 1.0))))) "None" true)
  (Class|PrimitiveComponent|AddAngularImpulseinDegrees (Variables|Default|GetBallSphere) (* (+ (* (Math|Vector|CrossProduct (Math|Vector|Normalize KickDirection) _returnvalue) SpinTop) (* _returnvalue SpinRight)) 1e+01) "None" true)
  (Default|CallOnBallKicked))

(fn ResetBall
  (params (SpawnTransform :type Transform) (bKeepSpin :type Boolean))
  (bind _returnvalue (Math|Vector|MakeVector 0.0 0.0 0.0))
  (Physics|SetSimulatePhysics (Variables|Default|GetBallSphere) false)
  (Transformation|SetActorTransform SpawnTransform false true)
  (Physics|SetPhysicsLinearVelocity (Variables|Default|GetBallSphere) _returnvalue false "None")
  (Class|PrimitiveComponent|SetPhysicsAngularVelocityinDegrees (Variables|Default|GetBallSphere) _returnvalue false "None")
  (Variables|Default|SetSpinAxis "0, 0, 0")
  (Variables|Default|SetSpinMagnitude 0.0)
  (Variables|Default|SetbMagnusActive false)
  (Variables|Default|SetbIsMoving false)
  (Physics|SetSimulatePhysics (Variables|Default|GetBallSphere) true))