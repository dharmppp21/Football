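; Player-controlled footballer with Enhanced Input movement, sprint, dribbling and charged gamepad kicks.
; A control zone collects slow balls, then each Tick blends the ball's horizontal physics velocity toward a guide point plus player velocity.
; Holding a face button charges the power meter, and release kicks with per-button power curve and lift.
; Right-button shots get aim assist toward a hard-coded goal location, with shoulder buttons adding finesse sidespin.
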(event OnComponentBeginOverlap(BallControlZone)
  (params (OverlappedComponent :type Primitive%20Component%20Object%20Reference) (OtherActor :type Actor%20Object%20Reference) (OtherComp :type Primitive%20Component%20Object%20Reference) (OtherBodyIndex :type Integer) (bFromSweep :type Boolean) (SweepResult :type Hit%20Result%20Structure%20%28by%20ref%29))
  (bind _asbp_football (Utilities|Casting|CastToBP_Football OtherActor))
  (if (and (< (Math|Vector|VectorLength (Transformation|GetVelocity _asbp_football)) 8e+02) (Variables|Default|GetbCanCollect))
    (Variables|Default|SetControlledBall _asbp_football)
    (Variables|Default|SetbHasBall true)))

(event OnComponentEndOverlap(BallControlZone)
  (params (OverlappedComponent :type Primitive%20Component%20Object%20Reference) (OtherActor :type Actor%20Object%20Reference) (OtherComp :type Primitive%20Component%20Object%20Reference) (OtherBodyIndex :type Integer))
  (Variables|Default|SetbCanCollect true))

(event Custom|TestForcePossession
  (bind _returnvalue (Actor|GetActorOfClass "/Game/Football/Blueprints/Ball/BP_Football.BP_Football_C"))
  (bind _asbp_football (Utilities|Casting|CastToBP_Football _returnvalue))
  (Variables|Default|SetControlledBall _asbp_football)
  (Variables|Default|SetbHasBall true)
  (Variables|Default|SetbCanCollect false))

(event Input|EnhancedActionEvents|EnhancedInputActionIA_Move
  (params (ActionValue :type Vector%202D%20Structure) (ElapsedSeconds :type Float%20%28double-precision%29) (TriggeredSeconds :type Float%20%28double-precision%29) (InputAction :type Input%20Action%20Object%20Reference :default "/Game/Football/Input/IA_Move.IA_Move"))
  (bind (_x _y) (Math|Vector2D|BreakVector2D ActionValue))
  (bind _returnvalue (Pawn|GetController))
  (bind _returnvalue_2 (Pawn|GetControlRotation _returnvalue :!class /Script/Engine.Controller))
  (bind _yaw (Math|Rotator|BreakRotator _returnvalue_2))
  (bind _returnvalue_3 (Math|Rotator|MakeRotator 0.0 0.0 _yaw))
  (Pawn|Input|AddMovementInput (Math|Vector|GetForwardVector _returnvalue_3) _y false)
  (Pawn|Input|AddMovementInput (Math|Vector|GetRightVector _returnvalue_3) _x false))

(event Input|EnhancedActionEvents|EnhancedInputActionIA_Look
  (params (ActionValue :type Vector%202D%20Structure) (ElapsedSeconds :type Float%20%28double-precision%29) (TriggeredSeconds :type Float%20%28double-precision%29) (InputAction :type Input%20Action%20Object%20Reference :default "/Game/Football/Input/IA_Look.IA_Look"))
  (bind (_x _y) (Math|Vector2D|BreakVector2D ActionValue))
  (Pawn|Input|AddControllerYawInput _x)
  (Pawn|Input|AddControllerPitchInput _y))

(event Input|EnhancedActionEvents|EnhancedInputActionIA_Sprint
  (params (ActionValue :type Boolean) (ElapsedSeconds :type Float%20%28double-precision%29) (TriggeredSeconds :type Float%20%28double-precision%29) (InputAction :type Input%20Action%20Object%20Reference :default "/Game/Football/Input/IA_Sprint.IA_Sprint"))
  (:Started
    (Variables|Default|SetbIsSprinting true)
    (Variables|/Script/Engine.CharacterMovementComponent|SetMaxWalkSpeed (Variables|Character|GetCharacterMovement) (Variables|Default|GetSprintSpeed)))
  (:Completed
    (Variables|Default|SetbIsSprinting false)
    (Variables|/Script/Engine.CharacterMovementComponent|SetMaxWalkSpeed (Variables|Character|GetCharacterMovement) (Variables|Default|GetWalkSpeed))
    (bind _returnvalue (Class|WidgetBlueprintLibrary|Create "/Game/Football/Blueprints/UI/WBP_PowerMeter.WBP_PowerMeter_C"))
    (bind _aswbp_power_meter (Utilities|Casting|CastToWBP_PowerMeter _returnvalue))
    (Variables|Default|SetPowerMeterRef _aswbp_power_meter)
    (UserInterface|Viewport|AddtoViewport _aswbp_power_meter 0)
    (Default|HideMeter _aswbp_power_meter)))

(event EventTick
  (params (DeltaSeconds :type Float%20%28single-precision%29))
  (bind _returnvalue (Transformation|GetActorLocation))
  (bind _returnvalue_2 (- "5270,0,150" _returnvalue))
  (Variables|Default|SetGoalVector _returnvalue_2)
  (Variables|Default|SetGoalDistanceM (* (Math|Vector|VectorLength _returnvalue_2) 0.01))
  (Variables|Default|SetShotPowerAlpha (Math|Float|Clamp(Float) (/ (- (Utilities|Time|GetTimeSeconds) (Variables|Default|GetShotChargeStartTime)) (Variables|Default|GetMaxShotChargeTime))))
  (Default|UpdatePower (Variables|Default|GetPowerMeterRef) (Variables|Default|GetShotPowerAlpha))
  (CallFunction|UpdateDribble))

(event EventBeginPlay
  (bind _asenhanced_input_local_player_subsystem (Utilities|Casting|CastToEnhancedInputLocalPlayerSubsystem (Class|SubsystemBlueprintLibrary|GetLocalPlayerSubSystemfromPlayerController (Game|GetPlayerController 0) "/Script/EnhancedInput.EnhancedInputLocalPlayerSubsystem")))
  (Input|AddMappingContext _asenhanced_input_local_player_subsystem "/Game/Football/Input/IMC_PracticeArena.IMC_PracticeArena" 10 "(bIgnoreAllPressedKeysUntilRelease=True,bForceImmediately=False,bNotifyUserSettings=False)")
  (Variables|/Script/Engine.CharacterMovementComponent|SetMaxWalkSpeed (Variables|Character|GetCharacterMovement) (Variables|Default|GetWalkSpeed))
  (bind _returnvalue (Class|WidgetBlueprintLibrary|Create "/Game/Football/Blueprints/UI/WBP_PowerMeter.WBP_PowerMeter_C"))
  (bind _aswbp_power_meter (Utilities|Casting|CastToWBP_PowerMeter _returnvalue))
  (Variables|Default|SetPowerMeterRef _aswbp_power_meter)
  (UserInterface|Viewport|AddtoViewport _aswbp_power_meter 0)
  (Default|HideMeter _aswbp_power_meter))

(event Input|GamepadEvents|GamepadFaceButtonRight
  (params (Key :type Key%20Structure :default "None"))
  (bind _shotpoweralpha (Variables|Default|GetShotPowerAlpha))
  (bind _shotpoweralpha_2 (Variables|Default|GetShotPowerAlpha))
  (bind _returnvalue (Math|Float|Power _shotpoweralpha_2 1.35))
  (bind _returnvalue_2 (Math|Float|Power _shotpoweralpha 1.35))
  (bind _returnvalue_3 (Math|Float|Lerp 0.22 1.0 _returnvalue))
  (bind _returnvalue_4 (Math|Float|Lerp 0.22 1.0 _returnvalue_2))
  (:Pressed
    (Variables|Default|SetbChargeFinesseR (Variables|Default|GetbRBHeld))
    (Variables|Default|SetbChargeFinesseL (Variables|Default|GetbLBHeld))
    (if (Variables|Default|GetbChargeFinesseR)
      (if (and (Utilities|IsValid (Variables|Default|GetControlledBall)) (<= (Transformation|GetDistanceTo (Variables|Default|GetControlledBall)) (Variables|Default|GetKickRange)))
        (Variables|Default|SetbIsChargingShot true :!label _label)
        (Variables|Default|SetShotChargeStartTime (Utilities|Time|GetTimeSeconds))
        (Default|ShowMeter (Variables|Default|GetPowerMeterRef)))
      (elif (Variables|Default|GetbChargeFinesseL)
        (if (and (Utilities|IsValid (Variables|Default|GetControlledBall)) (<= (Transformation|GetDistanceTo (Variables|Default|GetControlledBall)) (Variables|Default|GetKickRange)))
          (goto _label))
        (elif (and (Utilities|IsValid (Variables|Default|GetControlledBall)) (<= (Transformation|GetDistanceTo (Variables|Default|GetControlledBall)) (Variables|Default|GetKickRange)))
          (goto _label)))))
  (:Released
    (if (Variables|Default|GetbChargeFinesseR)
      (if (Variables|Default|GetbIsChargingShot)
        (Default|ApplyKick (Variables|Default|GetControlledBall) (Class|FootballLibrary|GetAimAssistedDirection (Transformation|GetActorForwardVector) (Variables|Default|GetGoalVector) (Variables|Default|GetGoalDistanceM)) (* 3.3e+03 _returnvalue_4) 0.3 (* 3.6e+02 _returnvalue_4) 0 0.0)
        (Variables|Default|SetbHasBall false)
        (Variables|Default|SetControlledBall 0)
        (Variables|Default|SetbCanCollect false)
        (Variables|Default|SetbIsChargingShot false)
        (Default|HideMeter (Variables|Default|GetPowerMeterRef) :!label _label_2))
      (elif (Variables|Default|GetbChargeFinesseL)
        (if (Variables|Default|GetbIsChargingShot)
          (Default|ApplyKick (Variables|Default|GetControlledBall) (Class|FootballLibrary|GetAimAssistedDirection (Transformation|GetActorForwardVector) (Variables|Default|GetGoalVector) (Variables|Default|GetGoalDistanceM)) (* 3.3e+03 _returnvalue_3) 0.3 (* -3.6e+02 _returnvalue_3) 0 0.0)
          (Variables|Default|SetbHasBall false)
          (Variables|Default|SetControlledBall 0)
          (Variables|Default|SetbCanCollect false)
          (Variables|Default|SetbIsChargingShot false)
          (goto _label_2))
        (elif (Variables|Default|GetbIsChargingShot)
          (Default|ApplyKick (Variables|Default|GetControlledBall) (Class|FootballLibrary|GetAimAssistedDirection (Transformation|GetActorForwardVector) (Variables|Default|GetGoalVector) (Variables|Default|GetGoalDistanceM)) (* 3.6e+03 (Math|Float|Lerp 0.2 1.0 (Math|Float|Power (Variables|Default|GetShotPowerAlpha) 1.25))) 0.26 0.0 0 0.0)
          (Variables|Default|SetbHasBall false)
          (Variables|Default|SetControlledBall 0)
          (Variables|Default|SetbCanCollect false)
          (Variables|Default|SetbIsChargingShot false)
          (goto _label_2))))))

(event Input|GamepadEvents|GamepadFaceButtonBottom
  (params (Key :type Key%20Structure :default "None"))
  (:Pressed
    (if (and (Utilities|IsValid (Variables|Default|GetControlledBall)) (<= (Transformation|GetDistanceTo (Variables|Default|GetControlledBall)) (Variables|Default|GetKickRange)))
      (Variables|Default|SetbIsChargingShot true)
      (Variables|Default|SetShotChargeStartTime (Utilities|Time|GetTimeSeconds))
      (Default|ShowMeter (Variables|Default|GetPowerMeterRef))))
  (:Released
    (if (Variables|Default|GetbIsChargingShot)
      (Default|ApplyKick (Variables|Default|GetControlledBall) (Transformation|GetActorForwardVector) (* 2.2e+03 (Math|Float|Lerp 0.2 1.0 (Math|Float|Power (Variables|Default|GetShotPowerAlpha) 1.1))) 0.03 0.0 0 -5.2e+02)
      (Variables|Default|SetbHasBall false)
      (Variables|Default|SetControlledBall 0)
      (Variables|Default|SetbCanCollect false)
      (Variables|Default|SetbIsChargingShot false)
      (Default|HideMeter (Variables|Default|GetPowerMeterRef)))))

(event Input|GamepadEvents|GamepadFaceButtonTop
  (params (Key :type Key%20Structure :default "None"))
  (:Pressed
    (if (and (Utilities|IsValid (Variables|Default|GetControlledBall)) (<= (Transformation|GetDistanceTo (Variables|Default|GetControlledBall)) (Variables|Default|GetKickRange)))
      (Variables|Default|SetbIsChargingShot true)
      (Variables|Default|SetShotChargeStartTime (Utilities|Time|GetTimeSeconds))
      (Default|ShowMeter (Variables|Default|GetPowerMeterRef))))
  (:Released
    (if (Variables|Default|GetbIsChargingShot)
      (Default|ApplyKick (Variables|Default|GetControlledBall) (Transformation|GetActorForwardVector) (* 2.6e+03 (Math|Float|Lerp 0.2 1.0 (Math|Float|Power (Variables|Default|GetShotPowerAlpha) 1.2))) 0.08 0.0 0 0.0)
      (Variables|Default|SetbHasBall false)
      (Variables|Default|SetControlledBall 0)
      (Variables|Default|SetbCanCollect false)
      (Variables|Default|SetbIsChargingShot false)
      (Default|HideMeter (Variables|Default|GetPowerMeterRef)))))

(event Input|GamepadEvents|GamepadRightShoulder
  (params (Key :type Key%20Structure :default "None"))
  (:Pressed
    (Variables|Default|SetbRBHeld true))
  (:Released
    (Variables|Default|SetbRBHeld false)))

(event Input|GamepadEvents|GamepadFaceButtonLeft
  (params (Key :type Key%20Structure :default "None"))
  (:Pressed
    (if (and (Utilities|IsValid (Variables|Default|GetControlledBall)) (<= (Transformation|GetDistanceTo (Variables|Default|GetControlledBall)) (Variables|Default|GetKickRange)))
      (Variables|Default|SetbIsChargingShot true)
      (Variables|Default|SetShotChargeStartTime (Utilities|Time|GetTimeSeconds))
      (Default|ShowMeter (Variables|Default|GetPowerMeterRef))))
  (:Released
    (if (Variables|Default|GetbIsChargingShot)
      (Default|ApplyKick (Variables|Default|GetControlledBall) (Transformation|GetActorForwardVector) (* 2.5e+03 (Math|Float|Lerp 0.19 1.0 (Math|Float|Power (Variables|Default|GetShotPowerAlpha) 1.15))) 0.75 0.0 0 0.0)
      (Variables|Default|SetbHasBall false)
      (Variables|Default|SetControlledBall 0)
      (Variables|Default|SetbCanCollect false)
      (Variables|Default|SetbIsChargingShot false)
      (Default|HideMeter (Variables|Default|GetPowerMeterRef)))))

(event Input|GamepadEvents|GamepadLeftShoulder
  (params (Key :type Key%20Structure :default "None"))
  (:Pressed
    (Variables|Default|SetbLBHeld true))
  (:Released
    (Variables|Default|SetbLBHeld false)))

(fn ConstructionScript)

(fn UpdateDribble
  (bind _controlledball (Variables|Default|GetControlledBall))
  (bind _ballguidepoint (Variables|Default|GetBallGuidePoint))
  (bind _controlledball_2 (Variables|Default|GetControlledBall))
  (bind _returnvalue (Transformation|GetWorldLocation _ballguidepoint))
  (bind _returnvalue_2 (Transformation|GetActorLocation _controlledball))
  (bind _ballsphere (Variables|/Game/Football/Blueprints/Ball/BP_Football.BP_Football_C|GetBallSphere _controlledball_2))
  (bind _returnvalue_3 (- _returnvalue _returnvalue_2))
  (if (Utilities|IsValid _controlledball)
    (if (Variables|Default|GetbHasBall)
      (bind _returnvalue_4 (Physics|GetPhysicsLinearVelocity _ballsphere "None"))
      (Physics|SetPhysicsLinearVelocity _ballsphere (Math|Vector|MakeVector (.X (Math|Vector|BreakVector (Math|Vector|Lerp(Vector) _returnvalue_4 (Math|Vector|ClampVectorSize (+ (* (Math|Vector|Normalize _returnvalue_3) (* (Math|Vector|VectorLength _returnvalue_3) (Variables|Default|GetDribbleStrength))) (Transformation|GetVelocity)) 0.0 (Variables|Default|GetMaxDribbleVelocity)) 0.4))) (.Y (Math|Vector|BreakVector (Math|Vector|Lerp(Vector) _returnvalue_4 (Math|Vector|ClampVectorSize (+ (* (Math|Vector|Normalize _returnvalue_3) (* (Math|Vector|VectorLength _returnvalue_3) (Variables|Default|GetDribbleStrength))) (Transformation|GetVelocity)) 0.0 (Variables|Default|GetMaxDribbleVelocity)) 0.4))) (.Z (Math|Vector|BreakVector _returnvalue_4))) false "None")
      (return)
      (else
        (return)))
    (else
      (return))))